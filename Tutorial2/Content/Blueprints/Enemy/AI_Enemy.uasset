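; Enemy pawn that walks a waypoint path and damages the objective it reaches, like a tower-defense creep.
; On BeginPlay it uses AI MoveTo toward the first TargetPoint tagged "Waypoint1".
; Tick checks distance to the current destination and, when close, advances through the Waypoint array with another AI MoveTo.
; Overlapping a BP_Objective subtracts health from it and destroys the enemy.
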(event Custom|MoveToNextWaypoint
  (bind _output_get (CallFunction|GetNextWaypoint))
  (bind _output_get_2 (Variables|Default|SetDestination (Transformation|GetActorLocation _output_get)))
  (AI|AIMoveTo self _output_get_2 0 5.0 false))

(event Collision|EventActorBeginOverlap
  (params (OtherActor :type Actor%20Object%20Reference))
  (bind _asbp_objective (Utilities|Casting|CastToBP_Objective OtherActor))
  (Variables|/Game/Blueprints/Objeective/BP_Objective.BP_Objective_C|Sethealth _asbp_objective (- (Variables|/Game/Blueprints/Objeective/BP_Objective.BP_Objective_C|Gethealth _asbp_objective) 1.0))
  (Actor|DestroyActor))

(event EventTick
  (params (DeltaSeconds :type Float%20%28single-precision%29))
  (if (<= (Math|Vector|Distance(Vector) (Variables|Default|GetDestination) (Transformation|GetActorLocation)) 1e+02)
    (if (< (Variables|Default|GetWaypointIndex) (Utilities|Array|Length (Variables|Default|GetWaypoint)))
      (CallFunction|MovetoNextWaypoint))))

(event EventBeginPlay
  (bind _objective (Variables|Default|GetObjective))
  (CallFunction|LocateObjective)
  (AI|AIMoveTo self "0, 0, 0" _objective 1e+01 false
    (:then
      (Variables|Default|SetDestination (Transformation|GetActorLocation _objective)))))

(fn ConstructionScript)

(fn LocateObjective
  (bind _outactors (Actor|GetAllActorsOfClasswithTag "/Script/Engine.TargetPoint" "Waypoint1"))
  (Variables|Default|SetObjective (Utilities|Array|Get(acopy) _outactors)))

(fn GetNextWaypoint
  (if (< (Variables|Default|GetWaypointIndex) (Utilities|Array|Length (Variables|Default|GetWaypoint)))
    (bind _output_get (Variables|Default|SetWaypointIndex (+ (Variables|Default|GetWaypointIndex) 1)))
    (return (Utilities|Array|Get(acopy) (Variables|Default|GetWaypoint) _output_get))))