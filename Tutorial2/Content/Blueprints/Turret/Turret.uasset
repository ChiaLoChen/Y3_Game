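; Turret Blueprint that spawns a Bullet actor on every Tick at the world transform of its Shoot component, with no rate limit.
; Spawning always proceeds regardless of collision.
; An unconnected line trace for WorldStatic objects along the forward vector is left in the graph, with a zero multiplier and unused result, and the construction script is empty.
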(event EventTick
  (params (DeltaSeconds :type Float%20%28single-precision%29))
  (Game|SpawnActorfromClass "/Game/Blueprints/Turret/Bullet.Bullet_C" (Transformation|GetWorldTransform (Variables|Default|Getshoot)) "AlwaysSpawn" "MultiplyWithRoot" 0 0))

(fn ConstructionScript)